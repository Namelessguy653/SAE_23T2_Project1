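; BP_Info_Slate is an environment info slate that displays a configurable title and description on a card.
; The construction script hides the InfoRoot hierarchy in game, disables collision on Card and InfoHolder, and applies the title and description text.
; A BlurMaterial flag picks between two slate card materials.
; Clicking the static mesh only prints a placeholder "Hello", and nothing in the graphs reveals the hidden info.
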(event `self.StaticMesh.OnClicked`
  (params (TouchedComponent :type "PrimitiveComponent Object Reference") (ButtonPressed :type "Key Structure"))
  (`KismetSystemLibrary.PrintString` "Hello"))

(fn `UserConstructionScript`
  (`SceneComponent.SetHiddenInGame` (`self.InfoRoot`) true true)
  (`PrimitiveComponent.SetCollisionEnabled` (`self.Card`) "NoCollision")
  (`PrimitiveComponent.SetCollisionEnabled` (`self.Info_Holder`) "NoCollision")
  (`TextRenderComponent.K2_SetText` (`self.Title`) (`self.titleText`))
  (`TextRenderComponent.K2_SetText` (`self.Description`) (`self.descriptionText`))
  (if (`self.bBlurMaterial?`)
    (`PrimitiveComponent.SetMaterial` (`self.Card`) 0 "/Game/Bazaar_Meshingun/Environment/Misc/MI_Card_Slate.MI_Card_Slate")
    (else
      (`PrimitiveComponent.SetMaterial` (`self.Card`) 0 "/Game/Bazaar_Meshingun/Environment/Misc/MI_Card_Slate_Plane.MI_Card_Slate_Plane"))))