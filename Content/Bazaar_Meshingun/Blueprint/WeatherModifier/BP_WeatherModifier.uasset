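; BP_WeatherModifier is a level actor that drives sand cover and tree and grass wind in materials through the MPC_Weather parameter collection.
; Its construction script destroys extra instances, then applies sand and wind enum presets only when they change, overwriting the variables and printing a notice.
; It then writes those variables to the collection, and repeats that write on BeginPlay so play mode matches.
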(event `self.ReceiveBeginPlay`
  ;[1 1 1] Sets weathers options in play mode
  (`self.ApplyToMaterialParameterCollection`))

(fn `ApplyToMaterialParameterCollection`
  ;[0.03646 0.03646 0.03646] Sand
  (`KismetMaterialLibrary.SetScalarParameterValue` "/Game/Bazaar_Meshingun/MPC/MPC_Weather.MPC_Weather" "SandAmount" (`self.sandAmount`))
  (`KismetMaterialLibrary.SetScalarParameterValue` "/Game/Bazaar_Meshingun/MPC/MPC_Weather.MPC_Weather" "SandAmonunt_Ground" (`self.sandAmount_Ground`))
  (`KismetMaterialLibrary.SetScalarParameterValue` "/Game/Bazaar_Meshingun/MPC/MPC_Weather.MPC_Weather" "Sand?" (`KismetMathLibrary.Conv_BoolToDouble` (`self.sand?`)))
  (`KismetMaterialLibrary.SetScalarParameterValue` "/Game/Bazaar_Meshingun/MPC/MPC_Weather.MPC_Weather" "SandTopMask" (`self.sandTopMask`))
  ;[0.03646 0.03646 0.03646] Wind
  (`KismetMaterialLibrary.SetScalarParameterValue` "/Game/Bazaar_Meshingun/MPC/MPC_Weather.MPC_Weather" "WindRotation_Tree" (`self.windRotation_Tree`))
  (`KismetMaterialLibrary.SetScalarParameterValue` "/Game/Bazaar_Meshingun/MPC/MPC_Weather.MPC_Weather" "WindSpeed_Tree" (`self.windSpeed_Tree`))
  (`KismetMaterialLibrary.SetScalarParameterValue` "/Game/Bazaar_Meshingun/MPC/MPC_Weather.MPC_Weather" "WindIntensity_Grass" (`self.windIntensity_Grass`))
  (`KismetMaterialLibrary.SetScalarParameterValue` "/Game/Bazaar_Meshingun/MPC/MPC_Weather.MPC_Weather" "WindSpeed_Grass" (`self.windSpeed_Grass`)))

(fn `ForceOneInstance`
  (bind _outactors (`GameplayStatics.GetAllActorsOfClass` "BP_WeatherModifier_C"))
  (if (> (`KismetArrayLibrary.Array_Length` _outactors) 1)
    (`KismetSystemLibrary.PrintString` "Only one instance of Weather Modifier is allowed in the level. The newly added actor was destroyed" true true (struct :`R` 1.0 :`B` 0.010267 :`A` 1.0) 7.0)
    (`self.K2_DestroyActor`)))

(fn `SetWeatherPresetParameters`
  (switch `/Game/Bazaar_Meshingun/Blueprint/WeatherModifier/E_WeatherPreset` (`self.weatherPreset`)
    (:`NewEnumerator0`
      ;[0.03646 0.03646 0.03646] Dry
      (set `self.sand?` false)
      (set `self.sandAmount` 0.0)
      (set `self.sandAmount_Ground` 0.0)
      (set `self.sandTopMask` 0.0))
    (:`NewEnumerator4`
      ;[1 0.734 0] Light Sandstorm
      (set `self.sand?` true)
      (set `self.sandAmount` 0.8)
      (set `self.sandAmount_Ground` 1.0)
      (set `self.sandTopMask` 0.0))
    (:`NewEnumerator3`
      ;[0.5938 0.4049 0] Heavy Sandstorm
      (set `self.sand?` true)
      (set `self.sandAmount` 1.2)
      (set `self.sandAmount_Ground` 1.75)
      (set `self.sandTopMask` 0.01))))

(fn `SetWindPresetParameters`
  (switch `/Game/Bazaar_Meshingun/Blueprint/WeatherModifier/E_WindPreset` (`self.windPreset`)
    (:`NewEnumerator0`
      (set `self.windSpeed_Tree` 0.0)
      (set `self.windRotation_Tree` 0.0)
      (set `self.windSpeed_Grass` 0.0)
      (set `self.windIntensity_Grass` 0.0))
    (:`NewEnumerator1`
      (set `self.windSpeed_Tree` 3.0)
      (set `self.windRotation_Tree` 0.5)
      (set `self.windSpeed_Grass` 1.0)
      (set `self.windIntensity_Grass` 2.0))
    (:`NewEnumerator2`
      (set `self.windSpeed_Tree` 4.0)
      (set `self.windRotation_Tree` 1.0)
      (set `self.windSpeed_Grass` 1.5)
      (set `self.windIntensity_Grass` 2.5))))

(fn `UserConstructionScript`
  (`self.ForceOneInstance`)
  (`self.WeatherPresetChanged` true)
  (`self.WindPresetChanged` true)
  (`self.ApplyToMaterialParameterCollection`))

(fn `WeatherPresetChanged`
  (params (bPrint :type Boolean :default true))
  (if (!= (`self.weatherPreset`) (`self.weatherPreset[DoNotChange]`))
    (set `self.weatherPreset[DoNotChange]` (`self.weatherPreset`))
    (`self.SetWeatherPresetParameters`)
    (if (`local.bPrint`)
      (`KismetSystemLibrary.PrintString` (`KismetStringLibrary.Concat_StrStr` (`KismetStringLibrary.Concat_StrStr` "[" (`KismetSystemLibrary.GetDisplayName` self) "]") " Weather preset have been changed to " (`KismetStringLibrary.Concat_StrStr` "'" (`|GetEnumeratorNameAsString` (`self.weatherPreset`)) "'") ". Some of material parameter variables in this blueprint are reset to match the weather preset. Click on ApplyPresetModifications to apply.") true true (struct :`R` 0.273651 :`G` 1.0 :`A` 1.0) 10.0))))

(fn `WindPresetChanged`
  (params (bPrint :type Boolean :default true))
  (if (!= (`self.windPreset`) (`self.windPreset[DoNotChange]`))
    (set `self.windPreset[DoNotChange]` (`self.windPreset`))
    (`self.SetWindPresetParameters`)
    (if (`local.bPrint`)
      (`KismetSystemLibrary.PrintString` (`KismetStringLibrary.Concat_StrStr` (`KismetStringLibrary.Concat_StrStr` "[" (`KismetSystemLibrary.GetDisplayName` self) "]") " Wind preset have been changed to " (`KismetStringLibrary.Concat_StrStr` "'" (`|GetEnumeratorNameAsString` (`self.windPreset`)) "'") ". Some of material parameter variables in this blueprint are reset to match the wind preset. Click on ApplyPresetModifications to apply.") true true (struct :`R` 0.273651 :`G` 1.0 :`A` 1.0) 10.0))))