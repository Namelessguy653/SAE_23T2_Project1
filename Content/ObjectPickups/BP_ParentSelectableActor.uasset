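; Base actor for selectable pickups, toggling a selection decal when selected or deselected.
; On BeginPlay, ShowWidget creates a WB_Tooltip for the first player controller and adds it to the viewport.
; HideWidget is empty, with an unconnected visibility call left in the graph, and IsSelected always returns false.
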(event `/Game/CharacterUI/BI_SelectActors.SelectMyActor`
  (`SceneComponent.SetVisibility` (`self.SelectedDecal`) true false))

(event `/Game/CharacterUI/BI_SelectActors.DeselectMyActor`
  (`SceneComponent.SetVisibility` (`self.SelectedDecal`) false false))

(event `self.ReceiveBeginPlay`
  (`self.ShowWidget`))

(event `ShowWidget`
  (bind _returnvalue (`|CreateWidget` "/Game/CharacterUI/WB_Tooltip.WB_Tooltip_C" (`GameplayStatics.GetPlayerController` 0)))
  (bind _output_get (set `self.WB_Tooltip` _returnvalue))
  (`UserWidget.AddToViewport` _output_get 0))

(event `HideWidget`)

(fn `isSelected?`
  (returns (`isSelected?` :type Boolean))
  (return false))

(fn `UserConstructionScript`)