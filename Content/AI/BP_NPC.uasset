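; Melee enemy NPC that chases the player on sight, attacks, and can be punched to death.
; Pawn sensing triggers an AI move to the player, then a delayed attack montage and damage on arrival.
; Overlaps with PlayerPunchCollision-tagged components apply the NPC's own BaseDamage to itself.
; Damage lowers clamped health, updates the health widget, and at zero plays a death animation and stops movement.
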(event `self.ReceiveBeginPlay`
  (`self.InitialiseHealth`))

(event `InitialiseHealth`
  (set `self.CurrentHealth` (`self.Max Health`)))

(event `self.PawnSensing.OnSeePawn`
  (params (Pawn :type "Pawn Object Reference"))
  (set `self.isSeeingPlayer` true)
  (`self.FollowPlayer`))

(event `FollowPlayer`
  (bind _returnvalue (`GameplayStatics.GetPlayerCharacter` 0))
  (set `self.CanAttack` true)
  (if (`self.isSeeingPlayer`)
    (`|AIMoveTo` self (0.0 0.0 0.0) _returnvalue
      (:`then`
        (if (`self.CanAttack`)
          (set `self.CanAttack` false)))
      (:`OnSuccess`
        (`KismetSystemLibrary.Delay` 1.1)
        (`self.PlayAnimMontage` "/Game/AI/AM_NPC.AM_NPC")
        (`GameplayStatics.ApplyDamage` _returnvalue (`self.Base Damage`))))))

(event `self.Capsule.OnComponentBeginOverlap`
  (params (OverlappedComponent :type "PrimitiveComponent Object Reference") (OtherActor :type "Actor Object Reference") (OtherComp :type "PrimitiveComponent Object Reference") (OtherBodyIndex :type Integer) (bFromSweep :type Boolean) (SweepResult :type "HitResult Structure (by ref)"))
  (if (`ActorComponent.ComponentHasTag` OtherComp "PlayerPunchCollision")
    (`GameplayStatics.ApplyDamage` self (`self.Base Damage`))))

(event `Death`
  (set `self.isDead` true)
  (`SkeletalMeshComponent.PlayAnimation` (`self.Mesh`) "/Game/AISoldier/Death.Death" false)
  (`MovementComponent.StopMovementImmediately` (`self.CharacterMovement`)))

(event `self.ReceiveAnyDamage`
  (params (Damage :type "Float (single-precision)") (DamageType :type "DamageType Object Reference") (InstigatedBy :type "Controller Object Reference") (DamageCauser :type "Actor Object Reference"))
  (`KismetSystemLibrary.PrintString` "I have taken damage... fuck")
  (if (not (`self.isDead`))
    (bind _output_get (set `self.CurrentHealth` (`KismetMathLibrary.FClamp` (- (`self.CurrentHealth`) Damage) 0.0 (`self.Max Health`))))
    (`/Game/AI/Health/AI_HealthWidget.UpdateHealthUI` (stale _output_get_2) _output_get (`self.Max Health`))
    (bind _asai_health_widget (cast `/Game/AI/Health/AI_HealthWidget` (`WidgetComponent.GetUserWidgetObject` (`self.Health Widget`))))
    (bind _output_get_2 (set `self.HealthWidgetRef` _asai_health_widget))
    (`ProgressBar.SetPercent` (`/Game/AI/Health/AI_HealthWidget.ProgressBar_39` _asai_health_widget) (- (`self.CurrentHealth`) 0.0))
    (if (== (`self.CurrentHealth`) 0.0)
      (`self.Death`))))

(fn `UpdateHealthBar`
  (set `self.Health` (`self.Max Health`))
  (return))

(fn `UserConstructionScript`)