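; Melee enemy NPC that chases the player once pawn sensing spots them.
; On reaching the player, it waits briefly, plays an attack montage and applies damage.
; Player punch overlaps apply damage to itself, but no damage handler lowers health and the timed death sequence's health check is unwired.
; A sphere overlap shows or hides its health widget, and the H key triggers ragdoll.
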(event `self.ReceiveBeginPlay`
  ;[1 1 1] Begin Play
  (`self.InitialiseHealth`)
  (cast `/Game/AI/Health/AI_HealthWidget` (`WidgetComponent.GetUserWidgetObject` (`self.Widget`)))
  (set `self.As AI Health Widget` (`self.HealthWidgetRef`)))

(event `InitialiseHealth`
  ;[1 1 1] Initialise Health
  (set `self.CurrentHealth` (`self.Max Health`)))

(event `self.PawnSensing.OnSeePawn`
  (params (Pawn :type "Pawn Object Reference"))
  ;[1 1 1] On See Pawn
  (set `self.isSeeingPlayer` true)
  (`self.FollowPlayer`))

(event `FollowPlayer`
  (bind _returnvalue (`GameplayStatics.GetPlayerCharacter` 0))
  ;[1 1 1] Follow Player
  (set `self.CanAttack` true)
  (if (`self.isSeeingPlayer`)
    (`|AIMoveTo` self (0.0 0.0 0.0) _returnvalue
      (:`then`
        (if (`self.CanAttack`)
          (set `self.CanAttack` false)))
      (:`OnSuccess`
        (`KismetSystemLibrary.Delay` 1.1)
        (`self.PlayAnimMontage` "/Game/AI/AM_NPC.AM_NPC")
        (`GameplayStatics.ApplyDamage` _returnvalue (`self.Base Damage`))))))

(event `self.Capsule.OnComponentBeginOverlap`
  (params (OverlappedComponent :type "PrimitiveComponent Object Reference") (OtherActor :type "Actor Object Reference") (OtherComp :type "PrimitiveComponent Object Reference") (OtherBodyIndex :type Integer) (bFromSweep :type Boolean) (SweepResult :type "HitResult Structure (by ref)"))
  ;[1 1 1] On Component Begin Overlap
  (if (`ActorComponent.ComponentHasTag` OtherComp "PlayerPunchCollision")
    (`GameplayStatics.ApplyDamage` self (`self.Base Damage`))))

(event `Death`
  ;[1 1 1] Death
  (set `self.isDead` true)
  (`SkeletalMeshComponent.PlayAnimation` (`self.Mesh`) "/Game/AISoldier/Death.Death" false)
  (`MovementComponent.StopMovementImmediately` (`self.CharacterMovement`))
  (`KismetSystemLibrary.Delay` 5.0)
  (`self.K2_DestroyActor`))

(event `self.Sphere Collision.OnComponentBeginOverlap`
  (params (OverlappedComponent :type "PrimitiveComponent Object Reference") (OtherActor :type "Actor Object Reference") (OtherComp :type "PrimitiveComponent Object Reference") (OtherBodyIndex :type Integer) (bFromSweep :type Boolean) (SweepResult :type "HitResult Structure (by ref)"))
  (cast `/Game/Paladin/Animations/BP_ThirdPersonCharacter` OtherActor)
  (`SceneComponent.SetVisibility` (`self.Widget`) true false))

(event `self.Sphere Collision.OnComponentEndOverlap`
  (params (OverlappedComponent :type "PrimitiveComponent Object Reference") (OtherActor :type "Actor Object Reference") (OtherComp :type "PrimitiveComponent Object Reference") (OtherBodyIndex :type Integer))
  (cast `/Game/Paladin/Animations/BP_ThirdPersonCharacter` OtherActor)
  (`SceneComponent.SetVisibility` (`self.Widget`) false false))

(event `self.ReceiveHit`
  (params (MyComp :type "PrimitiveComponent Object Reference") (Other :type "Actor Object Reference") (OtherComp :type "PrimitiveComponent Object Reference") (bSelfMoved :type Boolean) (HitLocation :type "Vector Structure") (HitNormal :type "Vector Structure") (NormalImpulse :type "Vector Structure") (Hit :type "HitResult Structure (by ref)"))
  (if (`ActorComponent.ComponentHasTag` OtherComp "RightHandCollision")
    _))

(event `Key|H`
  (params (Key :type "Key Structure"))
  (:`Pressed`
    (`self.Ragdoll/Death`)))

(fn `Ragdoll/Death`
  (`PrimitiveComponent.SetSimulatePhysics` (`self.Mesh`) true)
  (`CharacterMovementComponent.DisableMovement` (`self.CharacterMovement`)))

(fn `UpdateHealthBar`
  (set `self.Health` (`self.Max Health`))
  (return))

(fn `UserConstructionScript`)